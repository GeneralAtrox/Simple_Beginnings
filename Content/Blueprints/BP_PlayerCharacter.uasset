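; Player character Blueprint that moves a 2D flipbook sprite in four directions from the MoveUp and MoveLeft input axes.
; Each non-zero axis value sets the matching directional flipbook and adds movement input along world Z or Y.
; Only an exact value of 1 selects Up or Left, so other values show Down or Right.
; No idle flipbook is set, so the last one set persists.
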(event `InputAxis|MoveUp`
  (params (AxisValue :type "Float (single-precision)"))
  (bind _characterflipbook (`self.CharacterFlipbook`))
  ;[1 1 1] Character Movement + Flipbook Updating
  (if (!= AxisValue 0.0)
    (if (== AxisValue 1.0)
      (`PaperFlipbookComponent.SetFlipbook` _characterflipbook "/Game/Flipbooks/Player/Movement/Player_MoveUp.Player_MoveUp")
      (else
        (`PaperFlipbookComponent.SetFlipbook` _characterflipbook "/Game/Flipbooks/Player/Movement/Player_MoveDown.Player_MoveDown")))
    (`self.AddMovementInput` (0.0 0.0 1.0) AxisValue)))

(event `InputAxis|MoveLeft`
  (params (AxisValue :type "Float (single-precision)"))
  (bind _characterflipbook (`self.CharacterFlipbook`))
  ;[1 1 1] Character Movement + Flipbook Updating
  (if (!= AxisValue 0.0)
    (if (== AxisValue 1.0)
      (`PaperFlipbookComponent.SetFlipbook` _characterflipbook "/Game/Flipbooks/Player/Movement/Player_MoveLeft.Player_MoveLeft")
      (else
        (`PaperFlipbookComponent.SetFlipbook` _characterflipbook "/Game/Flipbooks/Player/Movement/Player_MoveRight.Player_MoveRight")))
    (`self.AddMovementInput` (0.0 1.0 0.0) AxisValue)))

(fn `UserConstructionScript`)